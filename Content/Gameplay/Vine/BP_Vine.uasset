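; BP_Vine is a vine actor that tells the player character when it is near and adjusts its movement around it.
; The Trigger volume sets IsNearVine on entry, then clears it and IsOnVine on exit and restores Walking mode.
; A separate ReleaseBox switches the character to Flying on entry and zeroes its velocity on exit.
; All logic is overlap-driven, with no Tick or input handling in this Blueprint.
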(event OnComponentBeginOverlap(Trigger)
  (params (OverlappedComponent :type Primitive%20Component%20Object%20Reference) (OtherActor :type Actor%20Object%20Reference) (OtherComp :type Primitive%20Component%20Object%20Reference) (OtherBodyIndex :type Integer) (bFromSweep :type Boolean) (SweepResult :type Hit%20Result%20Structure%20%28by%20ref%29))
  (bind _asplayer_character (Utilities|Casting|CastToPlayerCharacter OtherActor))
  (Variables|/Game/ThirdPersonBP/Blueprints/PlayerCharacter.PlayerCharacter_C|SetbIsNearVine _asplayer_character true))

(event OnComponentEndOverlap(Trigger)
  (params (OverlappedComponent :type Primitive%20Component%20Object%20Reference) (OtherActor :type Actor%20Object%20Reference) (OtherComp :type Primitive%20Component%20Object%20Reference) (OtherBodyIndex :type Integer))
  (bind _asplayer_character (Utilities|Casting|CastToPlayerCharacter OtherActor))
  (Variables|/Game/ThirdPersonBP/Blueprints/PlayerCharacter.PlayerCharacter_C|SetbIsNearVine _asplayer_character false)
  (Variables|/Game/ThirdPersonBP/Blueprints/PlayerCharacter.PlayerCharacter_C|SetbIsOnVine _asplayer_character false)
  (Pawn|Components|CharacterMovement|SetMovementMode (Variables|/Script/Engine.Character|GetCharacterMovement _asplayer_character) "MOVE_Walking" 0))

(event OnComponentBeginOverlap(ReleaseBox)
  (params (OverlappedComponent :type Primitive%20Component%20Object%20Reference) (OtherActor :type Actor%20Object%20Reference) (OtherComp :type Primitive%20Component%20Object%20Reference) (OtherBodyIndex :type Integer) (bFromSweep :type Boolean) (SweepResult :type Hit%20Result%20Structure%20%28by%20ref%29))
  (bind _asplayer_character (Utilities|Casting|CastToPlayerCharacter OtherActor))
  (Pawn|Components|CharacterMovement|SetMovementMode (Variables|/Script/Engine.Character|GetCharacterMovement _asplayer_character) "MOVE_Flying" 0))

(event OnComponentEndOverlap(ReleaseBox)
  (params (OverlappedComponent :type Primitive%20Component%20Object%20Reference) (OtherActor :type Actor%20Object%20Reference) (OtherComp :type Primitive%20Component%20Object%20Reference) (OtherBodyIndex :type Integer))
  (bind _asplayer_character (Utilities|Casting|CastToPlayerCharacter OtherActor))
  (Variables|/Script/Engine.MovementComponent|SetVelocity (Variables|/Script/Engine.Character|GetCharacterMovement _asplayer_character) (Math|Vector|MakeVector 0.0 0.0 0.0)))

(event EventBeginPlay)

(event Collision|EventActorBeginOverlap
  (params (OtherActor :type Actor%20Object%20Reference)))

(event EventTick
  (params (DeltaSeconds :type Float%20%28single-precision%29)))

(fn ConstructionScript)