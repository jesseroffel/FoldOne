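; BP_Finish is a level finish trigger that saves completion and advances the player to the next level.
; When the PlayerCharacter overlaps BoxTrigger while Active, it calls SetLevelComplete on FoldOneInstance with its level number.
; On a successful save it deactivates, shows the BP_LevelCompleted widget with the returned next level, then opens that level by name after a short delay.
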(event OnComponentBeginOverlap(BoxTrigger)
  (params (OverlappedComponent :type Primitive%20Component%20Object%20Reference) (OtherActor :type Actor%20Object%20Reference) (OtherComp :type Primitive%20Component%20Object%20Reference) (OtherBodyIndex :type Integer) (bFromSweep :type Boolean) (SweepResult :type Hit%20Result%20Structure%20%28by%20ref%29))
  (Utilities|Casting|CastToPlayerCharacter OtherActor)
  (if (Variables|LevelCompletion|GetbActive)
    ;[1 1 1] Load Next Level
    (bind _asfold_one_instance (Utilities|Casting|CastToFoldOneInstance (Game|GetGameInstance)))
    (bind (_saved _nextleveltoload) (Default|SetLevelComplete _asfold_one_instance (Variables|LevelCompletion|GetLevelNumberFinish)))
    (if _saved
      (Variables|LevelCompletion|SetbActive false)
      (bind _returnvalue (UserInterface|CreateWidget "/Game/UserInterface/BP_LevelCompleted.BP_LevelCompleted_C" (Game|GetPlayerController 0)))
      (UserInterface|Viewport|AddtoPlayerScreen _returnvalue)
      (bind _output_get (Variables|/Game/UserInterface/BP_LevelCompleted.BP_LevelCompleted_C|SetNextLevelLoading _returnvalue _nextleveltoload))
      (Utilities|FlowControl|Delay 5.0)
      (Game|OpenLevel(byName) (.PrimaryAssetName (Utilities|Struct|BreakPrimaryAssetId _output_get))))))

(fn ConstructionScript)