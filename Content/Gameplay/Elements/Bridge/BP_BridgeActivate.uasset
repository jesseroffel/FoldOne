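; BP_BridgeActivate is a bridge element that toggles between present and absent when its ActivateEffect event fires.
; On BeginPlay it hides the static mesh and disables its collision if IsVisible starts false.
; Each ActivateEffect call flips IsVisible, switching mesh visibility together with collision between none and query-and-physics.
; The construction script only calls the parent's.
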(event EventActivateEffect
  (bind _staticmesh (Variables|Default|GetStaticMesh))
  (if (Variables|Default|GetbIsVisible)
    (Rendering|SetVisibility _staticmesh false false)
    (Collision|SetCollisionEnabled _staticmesh "NoCollision")
    (Variables|Default|SetbIsVisible false)
    (else
      (Rendering|SetVisibility _staticmesh true false)
      (Collision|SetCollisionEnabled _staticmesh "QueryAndPhysics")
      (Variables|Default|SetbIsVisible true))))

(event EventBeginPlay
  (bind _staticmesh (Variables|Default|GetStaticMesh))
  (if (not (Variables|Default|GetbIsVisible))
    (Rendering|SetVisibility _staticmesh false false)
    (Collision|SetCollisionEnabled _staticmesh "NoCollision")))

(fn ConstructionScript
  (|CallParentFunction))