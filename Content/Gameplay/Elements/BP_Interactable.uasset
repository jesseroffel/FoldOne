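; Base interactable for element-gated gameplay objects, with default check, activation and follow-up events.
; UseInteractable fires ActivateEffect when active and the player's held element matches RequiredElement; the default effect sets that element on the player.
; Separate helpers remove or swap the player's element, and FollowUpEffect re-invokes UseInteractable when a follow-up is configured.
; GetPlayerReference lazily caches the first PlayerCharacter found.
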(event EventActivateEffect
  ;[1 1 1] Set the new Element
  (bind _playerreference (CallFunction|GetPlayerReference))
  (Default|SetElement _playerreference (Variables|ElementBehaviour|GetRequiredElement)))

(event EventUseInteractable
  (params (CharacterReference :type Player%20Character%20Object%20Reference%20%28by%20ref%29))
  ;[1 1 1] Default interaction check and execution
  (bind _result (CallFunction|CheckifElementMatch CharacterReference (Variables|ElementBehaviour|GetRequiredElement)))
  (if (and _result (Variables|Default|GetbIsActive))
    (CallFunction|ActivateEffect)))

(event EventFollowUpEffect
  ;[1 1 1] Default followup behaviour
  (if (and (Utilities|IsValid (Variables|Activation|GetFollowUpActor)) (Variables|Activation|GetbFollowUpAction))
    (bind _playerreference (CallFunction|GetPlayerReference))
    (CallFunction|UseInteractable _playerreference)))

(event EventDoActivationOnce
  ;[1 1 1] Remove Element
  (bind _playerreference (CallFunction|GetPlayerReference))
  (Default|RemoveElement _playerreference))

(fn ConstructionScript)

(fn GetPlayerReference
  (if (Utilities|IsValid (Variables|Default|GetPlayerReference))
    (return (Variables|Default|GetPlayerReference))
    (else
      (bind _outactors (Actor|GetAllActorsOfClass "/Game/ThirdPersonBP/Blueprints/PlayerCharacter.PlayerCharacter_C"))
      (if (Utilities|IsValid (Utilities|Array|Get(acopy) _outactors))
        (bind _output_get (Variables|Default|SetPlayerReference (Utilities|Array|Get(acopy) _outactors)))
        (return _output_get)))))

(fn TakeElementfromPlayer
  (params (PlayerReference :type Player%20Character%20Object%20Reference%20%28by%20ref%29) (CurrentElement :type E_ElementalType%20Enum%20%28by%20ref%29 :default "NewEnumerator0"))
  (Default|SetElement PlayerReference (Variables|ElementBehaviour|GetHeldElement))
  (Variables|ElementBehaviour|SetHeldElement CurrentElement))

(fn CheckifElementMatch
  (params (PlayerReference :type Player%20Character%20Object%20Reference%20%28by%20ref%29) (ElementType :type E_ElementalType%20Enum :default "NewEnumerator0"))
  (return (== (Variables|/Game/ThirdPersonBP/Blueprints/PlayerCharacter.PlayerCharacter_C|GetCurrentHeldElement PlayerReference) ElementType)))