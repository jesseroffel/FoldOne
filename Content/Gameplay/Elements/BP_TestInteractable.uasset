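; BP_TestInteractable is a test interactable, derived from a parent Blueprint, that trades elements with the player.
; UseInteractable fires ActivateEffect only when the interactable is active and CheckIfElementMatch accepts the character for RequiredElement.
; ActivateEffect branches on HeldElement, but both paths make the same SwitchElementWithPlayer call with the required and held elements.
; The construction script only calls its parent.
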(event EventUseInteractable
  (params (CharacterReference :type Player%20Character%20Object%20Reference%20%28by%20ref%29))
  ;[1 1 1] Default interaction check and execution
  (bind _result (CallFunction|CheckifElementMatch CharacterReference (Variables|Default|GetRequiredElement)))
  (if (and _result (Variables|Default|GetbIsActive))
    (CallFunction|ActivateEffect)))

(event EventActivateEffect
  (if (Utilities|Enum|Equal(Enum) "NewEnumerator0" (Variables|Default|GetHeldElement))
    (bind _playerreference (CallFunction|GetPlayerReference))
    (CallFunction|SwitchElementwithPlayer _playerreference (Variables|Default|GetRequiredElement) (Variables|Default|GetHeldElement))
    (else
      (bind _playerreference_2 (CallFunction|GetPlayerReference))
      (CallFunction|SwitchElementwithPlayer _playerreference_2 (Variables|Default|GetRequiredElement) (Variables|Default|GetHeldElement)))))

(fn ConstructionScript
  (|CallParentFunction))