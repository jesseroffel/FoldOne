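; BP_Tree is an interactable element Blueprint that changes the player's element when used.
; UseInteractable proceeds only if the tree is active and the character passes the RequiredElement match check, then branches on ActivateOnce.
; One-time activation gives the player the HeldElement and destroys the tree, while the repeatable effect sets the player's element to RequiredElement.
; The construction script only calls its parent.
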(event EventActivateEffect
  ;[1 1 1] Set the new Element
  (bind _playerreference (CallFunction|GetPlayerReference))
  (Default|SetElement _playerreference (Variables|Default|GetRequiredElement)))

(event EventUseInteractable
  (params (CharacterReference :type Player%20Character%20Object%20Reference%20%28by%20ref%29))
  ;[1 1 1] Default interaction check and execution
  (bind _result (CallFunction|CheckifElementMatch CharacterReference (Variables|Default|GetRequiredElement)))
  (if (and _result (Variables|Default|GetbIsActive))
    (if (Variables|Default|GetbActivateOnce)
      (CallFunction|DoActivationOnce)
      (else
        (CallFunction|ActivateEffect)))))

(event EventDoActivationOnce
  (bind _playerreference (CallFunction|GetPlayerReference))
  (Default|SetElement _playerreference (Variables|Default|GetHeldElement))
  (Actor|DestroyActor))

(fn ConstructionScript
  (|CallParentFunction))