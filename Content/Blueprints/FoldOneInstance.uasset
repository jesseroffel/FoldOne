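; FoldOneInstance is a game instance Blueprint that tracks level completion in a CompletedLevels array of completion flag, level name and map file.
; SetLevelComplete range-checks the level number, then flags the array's last entry, not the numbered one, as completed.
; It returns the map at the passed index as the next level.
; Saved reports only the range check; nothing is written to disk.
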(event EventInit)

(fn SetLevelComplete
  (params (LevelNumberCompleted :type Integer%20%28by%20ref%29))
  (bind _completedlevels (Variables|Default|GetCompletedLevels))
  (bind _completedlevels_2 (Variables|Default|GetCompletedLevels))
  (bind _returnvalue (Utilities|Array|Length _completedlevels_2))
  (bind _returnvalue_2 (- _returnvalue 1))
  (bind _output (Utilities|Array|Get(acopy) _completedlevels_2 _returnvalue_2))
  (bind (_bcompleted _levelname _mapfile) (Utilities|Struct|BreakCompletedLevels _output))
  (if (<= LevelNumberCompleted _returnvalue_2)
    (Utilities|Array|SetArrayElem _completedlevels_2 _returnvalue_2 (Utilities|Struct|MakeCompletedLevels true _levelname _mapfile))
    (if (<= LevelNumberCompleted (Utilities|Array|Length _completedlevels))
      (return true (.MapFile (Utilities|Struct|BreakCompletedLevels (Utilities|Array|Get(acopy) _completedlevels LevelNumberCompleted))))
      (else
        (Development|PrintString "All Levels complete")
        (return true "")))
    (else
      (return false ""))))